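; Openable door actor that swings open and shut in response to OnOpen and OnClose events from its OpenDoor component.
; A DoorSwing timeline drives a yaw offset combined with the rotation cached at BeginPlay, and closing reverses the same timeline.
; A timeline event track plays the door lock sound at the actor's location.
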(event `self.OpenDoor.OnOpen`
  (bind (_direction _openangle) (`Timeline|DoorSwing` :!label _label)
    (:`Update`
      (`self.K2_SetActorRotation` (`KismetMathLibrary.ComposeRotators` (`KismetMathLibrary.MakeRotator` 0.0 0.0 _openangle) (`self.InitialRotation`))))
    (:`Sound Timing`
      (`GameplayStatics.PlaySoundAtLocation` "/Game/Audio/door-lock.door-lock" (`self.K2_GetActorLocation`)))))

(event `self.OpenDoor.OnClose`
  (goto _label :!via `Reverse`))

(event `self.ReceiveBeginPlay`
  (set `self.InitialRotation` (`self.K2_GetActorRotation`)))

(fn `UserConstructionScript`)